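; Slot-based inventory that stores item stacks in a Content array and handles adding, removing and transferring items between inventories.
; Adding fills matching stacks before empty slots, using data table stack limits and per-slot allowed-item lists.
; Transfers merge or swap slots and notify both inventories through OnInventoryUpdated, or restore the source slot widget's visuals when rejected.
; A block flag disables all three operations, and debug helpers print slot contents.
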(event `self.ReceiveBeginPlay`
  (`KismetArrayLibrary.Array_Resize` (`self.Content`) (`self.InventorySize`)))

(event `Update`
  (`self.OnInventoryUpdated`))

(fn `AddToInventory`
  (params (ItemID :type Name) (Quantity :type Integer))
  (returns (Success :type Boolean) (QuantityRemaining :type Integer))
  (locals (QuantityRemain :type Integer) (HasFailed :type Boolean))
  (bind _output_get (set `local.QuantityRemain` Quantity))
  (if (not (`self.IsBlocked`))
    (while (and (> _output_get 0) (not (`local.HasFailed`)))
      (bind (_slotindex _slotisfound) (`self.FindSlot` (`local.ItemID`)))
      (if _slotisfound
        (`self.AddToStack` _slotindex 1)
        (`/Engine/EditorBlueprintResources/StandardMacros.DecrementInt` (`local.QuantityRemain`))
        (elif (`self.AnyEmptySlotsAvaiable`)
          (bind _success (`self.CreateNewStack` (`local.ItemID`) 1))
          (if _success
            (`/Engine/EditorBlueprintResources/StandardMacros.DecrementInt` (`local.QuantityRemain`))
            (else
              (set `local.HasFailed` true)))
          (else
            (set `local.HasFailed` true)))))
    (return (not (`local.HasFailed`)) (`local.QuantityRemain`))
    (else
      (return (not (`local.HasFailed`)) (`local.QuantityRemain`)))))

(fn `AddToStack`
  (params (Index :type Integer) (Quantity :type Integer))
  (bind (_output_itemid _output_quantity _output_itemtypes) (break `/Game/InventorySystem/SlotStruct` (`|GetArrayItem` (`self.Content`) Index)))
  (`KismetArrayLibrary.Array_Set` (`self.Content`) Index (make `/Game/InventorySystem/SlotStruct` _output_itemid (+ _output_quantity Quantity) _output_itemtypes)))

(fn `AnyEmptySlotsAvaiable`
  (returns (HasEmptySlot :type Boolean) (EmptyIndex :type Integer))
  (for (_array_element _array_index) (`self.Content`)
    (if (== (`.Quantity_5_034EA8CE41C925DA0A3BD2817C871E1F` (break `/Game/InventorySystem/SlotStruct` _array_element)) 0)
      (return true _array_index)))
  (return false -1))

(fn `CreateNewStack`
  (params (ItemID :type Name) (Quantity :type Integer))
  (returns (Success :type Boolean))
  (bind (_hasemptyslot _emptyindex) (`self.AnyEmptySlotsAvaiable`))
  (if _hasemptyslot
    (for _array_element (`self.Content`)
      (bind (_itemid _quantity _itemtypes) (break `/Game/InventorySystem/SlotStruct` _array_element))
      (if (== (`|GetArrayItem` _itemtypes) "None")
        (`KismetArrayLibrary.Array_Set` (`self.Content`) _emptyindex (make `/Game/InventorySystem/SlotStruct` (`local.ItemID`) (`local.Quantity`) (`.ItemTypes_11_4893CB9A4B53072036A22B97ADE17BC0` (break `/Game/InventorySystem/SlotStruct` (`|GetArrayItem` (`self.Content`) _emptyindex)))))
        (return true)
        (else
          (for _array_element_2 _itemtypes
            (if (== (`local.ItemID`) _array_element_2)
              (`KismetArrayLibrary.Array_Set` (`self.Content`) _emptyindex (make `/Game/InventorySystem/SlotStruct` (`local.ItemID`) (`local.Quantity`) _itemtypes))
              (return true)))
          (return false))))
    (else
      (return false))))

(fn `FindSlot`
  (params (ItemID :type Name))
  (returns (SlotIndex :type Integer) (SlotIsFound :type Boolean))
  (for (_array_element _array_index) (`self.Content`)
    (bind (_itemid _quantity _itemtypes) (break `/Game/InventorySystem/SlotStruct` _array_element))
    (if (== _itemid ItemID)
      (if (< _quantity (`self.GetMaxStackSize` ItemID))
        (if (== (`|GetArrayItem` _itemtypes) "None")
          (return _array_index true)
          (else
            (for _array_element_2 _itemtypes
              (if (== (`local.ItemID`) _array_element_2)
                (return _array_index true)))
            (return -1 false))))))
  (return -1 false))

(fn `ForDEBUG_PrintContent`
  (for _array_element (`self.Content`)
    (bind (_itemid _quantity) (break `/Game/InventorySystem/SlotStruct` _array_element))
    (`KismetSystemLibrary.PrintText` (`|FormatText` "{0}: {1}" _quantity _itemid))))

(fn `ForDEBUG_PrintZeroElementInSlotType`
  (if (== (`KismetArrayLibrary.Array_Length` (`self.Content`)) 1)
    (for _array_element (`self.Content`)
      (`KismetSystemLibrary.PrintString` (`KismetTextLibrary.Conv_TextToString` (`|FormatText` "{0}: {1}" (`KismetTextLibrary.Conv_StringToText` (`KismetSystemLibrary.GetDisplayName` self)) (`KismetStringLibrary.Conv_NameToString` (`|GetArrayItem` (`.ItemTypes_11_4893CB9A4B53072036A22B97ADE17BC0` (break `/Game/InventorySystem/SlotStruct` _array_element)))))) true true (struct :`G` 0.66 :`B` 1.0 :`A` 1.0) 10.0))))

(fn `GetMaxStackSize`
  (params (ItemID :type Name))
  (returns (StackSize :type Integer))
  (bind _returnvalue (`|GetDataTableRow` "/Game/InventorySystem/ItemDataTable.ItemDataTable" ItemID)
    (:`then`
      (return (`.StackSize_16_13F2EEB846EDDD8ACBD96ABA4FE30D39` (break `/Game/InventorySystem/ItemStruct` _returnvalue))))
    (:`RowNotFound`
      (return -1))))

(fn `RemoveItem`
  (params (ItemID :type Name) (Quantity :type Integer))
  (returns (Success :type Boolean))
  (locals (ArrayIndexes :type "Array of Integer") (ItemsSum :type Integer) (QuantityRemain :type Integer))
  (bind _content (`self.Content`))
  (bind _content_2 (`self.Content`))
  (bind _quantityremain (`local.QuantityRemain`))
  (set `local.QuantityRemain` Quantity)
  (if (not (`self.IsBlocked`))
    (for (_array_element _array_index) (`self.Content`)
      (if (== (break `/Game/InventorySystem/SlotStruct` _array_element) ItemID)
        (`KismetArrayLibrary.Array_Add` (`local.ArrayIndexes`) _array_index)
        (set `local.ItemsSum` (+ (`.Quantity_5_034EA8CE41C925DA0A3BD2817C871E1F` (break `/Game/InventorySystem/SlotStruct` _array_element)) (`local.ItemsSum`)))))
    (if (>= (`local.ItemsSum`) (`local.QuantityRemain`))
      (for _array_element_2 (`local.ArrayIndexes`)
        (bind (_output_itemid _output_quantity _output_itemtypes) (break `/Game/InventorySystem/SlotStruct` (`|GetArrayItem` _content _array_element_2)))
        (if (>= _output_quantity _quantityremain)
          (`KismetArrayLibrary.Array_Set` _content _array_element_2 (make `/Game/InventorySystem/SlotStruct` _output_itemid (- _output_quantity _quantityremain) _output_itemtypes))
          (`self.Update`)
          (return true)
          (else
            (bind _returnvalue (`|GetDataTableRow` "/Game/InventorySystem/ItemDataTable.ItemDataTable" _output_itemid)
              (:`then`
                (bind (_output_itemid_2 _output_quantity_2 _output_itemtypes_2) (break `/Game/InventorySystem/SlotStruct` (`|GetArrayItem` _content_2 _array_element_2)))
                (`KismetArrayLibrary.Array_Set` _content_2 _array_element_2 (make `/Game/InventorySystem/SlotStruct` _output_itemid_2 (- _output_quantity_2 (`.StackSize_16_13F2EEB846EDDD8ACBD96ABA4FE30D39` (break `/Game/InventorySystem/ItemStruct` _returnvalue))) _output_itemtypes_2))
                (set `local.QuantityRemain` (- (`local.QuantityRemain`) (`.StackSize_16_13F2EEB846EDDD8ACBD96ABA4FE30D39` (break `/Game/InventorySystem/ItemStruct` _returnvalue)))))
              (:`RowNotFound`
                (return false))))))
      (`self.Update`)
      (return true)
      (else
        (return false)))
    (else
      (return false))))

(fn `SetBlockInventory`
  (params (Block :type Boolean))
  (set `self.IsBlocked` Block))

(fn `TransferSlots`
  (params (SourceIndex :type Integer) (DestinationIndex :type Integer) (SourceInventory :type "/Game/InventorySystem/InventorySystemBP Object Reference") (SourceSlot :type "/Game/Blueprints/HUD/Inventory/InventorySlot Object Reference"))
  (locals (LocalSlotData :type "/Game/InventorySystem/SlotStruct Structure"))
  (bind _content (`self.Content`))
  (bind _sourceslot (`local.SourceSlot`))
  (bind (_localslotdata_itemid _localslotdata_quantity) (break `/Game/InventorySystem/SlotStruct` (`local.LocalSlotData`)))
  (bind (_localslotdata_itemid_2 _localslotdata_quantity_2 _localslotdata_itemtypes) (break `/Game/InventorySystem/SlotStruct` (`local.LocalSlotData`)))
  (bind _content_2 (`self.Content`))
  (bind _destinationindex (`local.DestinationIndex`))
  (bind (_itemid _quantity) (break `/Game/InventorySystem/SlotStruct` (`local.LocalSlotData`)))
  (bind _itemid_2 (break `/Game/InventorySystem/SlotStruct` (`local.LocalSlotData`)))
  (bind _stacksize (`self.GetMaxStackSize` _localslotdata_itemid))
  (bind (_output_itemid _output_quantity) (break `/Game/InventorySystem/SlotStruct` (`|GetArrayItem` (`self.Content`) (`local.DestinationIndex`))))
  (bind (_output_itemid_2 _output_quantity_2 _output_itemtypes) (break `/Game/InventorySystem/SlotStruct` (`|GetArrayItem` _content_2 _destinationindex)))
  (bind (_itemid_3 _quantity_2 _itemtypes) (break `/Game/InventorySystem/SlotStruct` (`|GetArrayItem` (`self.Content`) (`local.DestinationIndex`))))
  (bind (_itemid_4 _quantity_3) (break `/Game/InventorySystem/SlotStruct` (`|GetArrayItem` (`self.Content`) (`local.DestinationIndex`))))
  (bind _returnvalue (+ _localslotdata_quantity _output_quantity))
  (bind _returnvalue_2 (- _returnvalue _stacksize))
  (bind _returnvalue_3 (> _returnvalue_2 0))
  (set `local.LocalSlotData` (`|GetArrayItem` (`/Game/InventorySystem/InventorySystemBP.Content` SourceInventory) SourceIndex))
  (if (not (`self.IsBlocked`))
    (if (!= (`|GetArrayItem` _itemtypes) "None")
      (if (`KismetArrayLibrary.Array_Contains` _itemtypes _itemid_2)
        (if (== _itemid_2 _itemid_3) :!label _label
          (`KismetArrayLibrary.Array_Set` (`/Game/InventorySystem/InventorySystemBP.Content` (`local.SourceInventory`)) (`local.SourceIndex`) (make `/Game/InventorySystem/SlotStruct` (select `bool` _returnvalue_3 :`true` _localslotdata_itemid_2) (`KismetMathLibrary.Clamp` _returnvalue_2 0 _stacksize) _localslotdata_itemtypes))
          (`KismetArrayLibrary.Array_Set` _content_2 _destinationindex (make `/Game/InventorySystem/SlotStruct` _localslotdata_itemid_2 (select `bool` _returnvalue_3 :`false` _returnvalue :`true` _stacksize) _output_itemtypes))
          (`self.Update`)
          (`self.Update` (`local.SourceInventory`))
          (else
            (`KismetArrayLibrary.Array_Set` (`/Game/InventorySystem/InventorySystemBP.Content` (`local.SourceInventory`)) (`local.SourceIndex`) (make `/Game/InventorySystem/SlotStruct` _itemid_4 _quantity_3 (`.ItemTypes_11_4893CB9A4B53072036A22B97ADE17BC0` (break `/Game/InventorySystem/SlotStruct` (`local.LocalSlotData`)))))
            (`KismetArrayLibrary.Array_Set` _content (`local.DestinationIndex`) (make `/Game/InventorySystem/SlotStruct` _itemid _quantity (`.ItemTypes_11_4893CB9A4B53072036A22B97ADE17BC0` (break `/Game/InventorySystem/SlotStruct` (`|GetArrayItem` _content (`local.DestinationIndex`))))))
            (`self.Update`)
            (`self.Update` (`local.SourceInventory`))))
        (else
          (`Border.SetBrushColor` (`/Game/Blueprints/HUD/Inventory/InventorySlot.QuantityRarityBorder` _sourceslot) (`/Game/Blueprints/HUD/Inventory/InventorySlot.ItemRarity` _sourceslot) :!label _label_2)
          (`Border.SetBrushColor` (`/Game/Blueprints/HUD/Inventory/InventorySlot.RarityBorder` _sourceslot) (`/Game/Blueprints/HUD/Inventory/InventorySlot.ItemRarity` _sourceslot))
          (`Widget.SetVisibility` (`/Game/Blueprints/HUD/Inventory/InventorySlot.ItemIcon` _sourceslot) "Visible")
          (`Widget.SetVisibility` (`/Game/Blueprints/HUD/Inventory/InventorySlot.QuantityBox` _sourceslot) "Visible")))
      (else
        (goto _label)))
    (else
      (goto _label_2))))