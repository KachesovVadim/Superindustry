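; Solar panel mechanism that supplies energy to oxygen tankers in the level.
; Every Tick it finds all OxygenTankerBP actors, casts them to Mechanism into TargetArray, passes that array to GiveEnergy, then clears it.
; The lookup is a world-wide class search each frame, with no range or sunlight check in this graph.
; Similar branches for PocketStotage and PocketDrill exist but are disconnected and never run.
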(event `self.ReceiveTick`
  (params (DeltaSeconds :type "Float (single-precision)"))
  (bind _target_array (`self.Target Array`))
  (`|ExecutionSequence`
    (:`then_0`
      (bind _outactors (`GameplayStatics.GetAllActorsOfClass` "/Game/Blueprints/Mechanisms/OxygenTankerBP.OxygenTankerBP_C"))
      (for _array_element _outactors
        (`KismetArrayLibrary.Array_Add` _target_array (cast `Mechanism` _array_element :!pure true)))
      (`self.GiveEnergy` _target_array)
      (`KismetArrayLibrary.Array_Clear` (`self.Target Array`)))))

(fn `UserConstructionScript`)