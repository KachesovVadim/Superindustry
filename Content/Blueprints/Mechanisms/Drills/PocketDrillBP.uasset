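; Pocket drill machine that mines ores over time into its ore inventory, using up drill pipes.
; Each tick, WorkBP calls Work and accumulates delta time up to a threshold scaled by mining level.
; Each completed cycle consumes one pipe and picks an ore from that level's percentage ranges, re-rolling for every comparison.
; It pauses when work or pipe removal fails, and exposes the remaining cycle fraction.
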(event `self.ReceiveBeginPlay`)

(event `self.ReceiveTick`
  (params (DeltaSeconds :type "Float (single-precision)"))
  (bind _inventory_ores (`self.Inventory-ores`))
  (set `self.DelatsSecs` DeltaSeconds)
  (bind _orename (`self.WorkBP` (`self.CurrentMiningLevel`)))
  (if (!= _orename "None")
    (`/Game/InventorySystem/InventorySystemBP.AddToInventory` _inventory_ores _orename 1)
    (`/Game/InventorySystem/InventorySystemBP.Update` _inventory_ores)))

(fn `GetMiningStatus`
  (returns (Percent :type "Float (double-precision)"))
  (bind _returnvalue (* (`self.CurrentMiningLevel`) (`self.MiningMultiplier`)))
  (return (/ (- _returnvalue (`self.TicksMined`)) _returnvalue)))

(fn `SetCurrentMiningLevel`
  (params (MiningLevel :type Integer))
  (set `self.CurrentMiningLevel` MiningLevel))

(fn `UserConstructionScript`)

(fn `WorkBP`
  (params (MiningLevel :type Integer))
  (returns (OreName :type Name))
  (locals (TotalRarityOnLevel :type "Float (double-precision)"))
  (bind _returnvalue (`KismetMathLibrary.RandomIntegerInRange` 1 100))
  (bind (_output_height _output_ores) (break `/Game/Blueprints/Mechanisms/Drills/MiningStruct` (`|GetArrayItem` (`self.MiningList`) MiningLevel)))
  (bind _returnvalue_2 (* (`self.CurrentMiningLevel`) (`self.MiningMultiplier`)))
  (bind _returnvalue_3 (`self.Work` _returnvalue_2))
  (if _returnvalue_3
    (set `self.TicksMined` (+ (`self.DelatsSecs`) (`self.TicksMined`)))
    (if (> (`self.TicksMined`) _returnvalue_2)
      (bind _success (`/Game/InventorySystem/InventorySystemBP.RemoveItem` (`self.Inventory-pipes`) "drillpipe" 1))
      (if _success
        (set `self.TicksMined` 0.0)
        (for _array_element _output_ores
          (if (and (<= (`.OreMiningRangeStart_8_385EAC994A62DA0CA39B35B510585B7E` (break `/Game/Blueprints/Mechanisms/Drills/OreStruct` _array_element)) _returnvalue) (>= (`.OreMiningRangeEnd_10_C4D15B0A4777A79B0BB44288A9DFBA7E` (break `/Game/Blueprints/Mechanisms/Drills/OreStruct` _array_element)) _returnvalue))
            (return (break `/Game/Blueprints/Mechanisms/Drills/OreStruct` _array_element))))
        (return "None")
        (else
          (`self.SetPause` true)
          (return "None")))
      (else
        (return "None")))
    (else
      (`self.SetPause` true)
      (return "None"))))