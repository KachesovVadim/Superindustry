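; BP_AuraFactor tracks an aura mode (Calm, Defense, Attack or OFF) and decides which parameters are displayed for it.
; ChangeAuraMode stores the new mode and rebuilds ParamsToDisplay, pairing one mode-specific parameter with Mana.
; Calm, Defense and OFF then fire OnParamsChanged to notify listeners, while the Attack branch updates the list without firing it.
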(event `ChangeParamsToDisplay`
  (`KismetArrayLibrary.Array_Clear` (`self.ParamsToDisplay`))
  (switch `/Game/Blueprints/Aura/AuraModes` (`self.AuraMode`)
    (:`NewEnumerator0`
      (set `self.ParamsToDisplay` (`|MakeArray` (`self.Сoncentration`) (`self.Mana`)))
      (`self.OnParamsChanged` :!label _label))
    (:`NewEnumerator1`
      (set `self.ParamsToDisplay` (`|MakeArray` (`self.ShieldsState`) (`self.Mana`)))
      (goto _label))
    (:`NewEnumerator2`
      (set `self.ParamsToDisplay` (`|MakeArray` (`self.AuraState`) (`self.Mana`)))
      (goto _label))
    (:`NewEnumerator3`
      (set `self.ParamsToDisplay` (`|MakeArray` (`self.AttackState`) (`self.Mana`))))))

(fn `ChangeAuraMode`
  (params (AuraMode :type "/Game/Blueprints/Aura/AuraModes Enum" :default "NewEnumerator0"))
  (set `self.AuraMode` AuraMode)
  (`self.ChangeParamsToDisplay`))

(fn `UserConstructionScript`)