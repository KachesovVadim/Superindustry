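; MainHUD is a HUD Blueprint that manages the game's in-game info, journal and main menu widgets.
; BeginPlay creates the InGameInfo widget without adding it to the viewport and loads the initial journal note text from row "1" of NoteTable.
; JournalSense toggles the journal, disabling character input while it shows and building a fresh widget on each opening.
; ShowMainMenu displays a new main menu, and SetJournalNoteText replaces the stored note.
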(event `self.ReceiveBeginPlay`
  (bind _returnvalue (`|CreateWidget` "/Game/Blueprints/HUD/InGameInfo.InGameInfo_C" (`GameplayStatics.GetPlayerController` 0)))
  (set `self.InGameInfo` _returnvalue)
  (bind _returnvalue_2 (`|GetDataTableRow` "/Game/StorySystem/NoteTable.NoteTable" "1")
    (:`then`
      (set `self.JournalNoteText` (break `/Game/StorySystem/NoteStruct` _returnvalue_2)))))

(event `JournalSense`
  (bind _journal (`self.Journal`)
    (:`then`
      (if (`Widget.IsInViewport` _journal)
        (`Widget.RemoveFromParent` _journal)
        (`SuperIndustryCharacter.Enable_Input` (cast `/Game/Blueprints/BP_ThirdPersonCharacter` (`GameplayStatics.GetPlayerCharacter` 0) :!pure true))
        (else
          (bind _returnvalue (`|CreateWidget` "/Game/StorySystem/Journal.Journal_C" :!label _label))
          (bind _output_get (set `self.Journal` _returnvalue))
          (`UserWidget.AddToViewport` _output_get 0)
          (`SuperIndustryCharacter.Disable_Input` (cast `/Game/Blueprints/BP_ThirdPersonCharacter` (`GameplayStatics.GetPlayerCharacter` 0) :!pure true)))))
    (:`else`
      (goto _label))))

(event `ShowMainMenu`
  (bind _returnvalue (`|CreateWidget` "/Game/Blueprints/HUD/MainMenu/MainMenu.MainMenu_C"))
  (`UserWidget.AddToViewport` _returnvalue 0))

(fn `SetJournalNoteText`
  (params (Text :type Text))
  (set `self.JournalNoteText` Text))

(fn `UserConstructionScript`)