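; BP_ExtraFog is an overlap-triggered actor, named as extra fog, that switches the player's aura mode while the player is inside it.
; It reacts only when the overlapping actor is the player's BP_ThirdPersonCharacter.
; Begin and end overlap call ChangeAuraMode on the AuraFactor held by MyGameInstance, setting one mode on entry and another on exit.
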(event `self.ReceiveActorBeginOverlap`
  (params (OtherActor :type "Actor Object Reference"))
  (if (== (cast `/Game/Blueprints/BP_ThirdPersonCharacter` (`GameplayStatics.GetPlayerCharacter` 0) :!pure true) OtherActor)
    (`/Game/Blueprints/Aura/BP_AuraFactor.ChangeAuraMode` (`/Game/Blueprints/MyGameInstance.AuraFactor` (cast `/Game/Blueprints/MyGameInstance` (`GameplayStatics.GetGameInstance`) :!pure true)) "NewEnumerator1")))

(event `self.ReceiveActorEndOverlap`
  (params (OtherActor :type "Actor Object Reference"))
  (if (== (cast `/Game/Blueprints/BP_ThirdPersonCharacter` (`GameplayStatics.GetPlayerCharacter` 0) :!pure true) OtherActor)
    (`/Game/Blueprints/Aura/BP_AuraFactor.ChangeAuraMode` (`/Game/Blueprints/MyGameInstance.AuraFactor` (cast `/Game/Blueprints/MyGameInstance` (`GameplayStatics.GetGameInstance`) :!pure true)) "NewEnumerator0")))

(fn `UserConstructionScript`)